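; Per-wheel suspension component for the drift car owned by BP_MainDirftController, simulating a raycast spring.
; Each tick a line trace finds the ground, and a spring-damper force from the compression and its rate is applied to the car's root.
; The child wheel mesh and optional emitter follow the hit point.
; Wheels spin with car speed; rear-drive wheels stop under handbrake and otherwise add spin from the Arrow's yaw.
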(event Custom|Set%20Spring%20Values
  (params (SpringCoeficient :type Float%20%28double-precision%29) (DampingCoeficient :type Float%20%28double-precision%29))
  (Variables|Default|SetSpringCoeficient SpringCoeficient)
  (Variables|Default|SetDampingCoeficient DampingCoeficient))

(event Custom|Set%20Wheel%20Offset
  (params (WheelMeshOffset :type Float%20%28double-precision%29) (WheelPosition :type Float%20%28double-precision%29))
  (Variables|Default|SetWheelMeshOffset WheelMeshOffset)
  (Variables|Default|SetWheelPosition WheelPosition))

(event EventBeginPlay
  (bind _asbp_main_dirft_controller (Utilities|Casting|CastToBP_MainDirftController (Components|GetOwner)))
  (Variables|Default|SetPlayerRef _asbp_main_dirft_controller)
  (Variables|Default|SetWheelRef (Components|GetChildComponent 0))
  (Variables|Default|SetOriginalWheelPos (Variables|Default|GetRelativeLocation)))

(event EventTick
  (params (DeltaSeconds :type Float%20%28single-precision%29))
  (bind _returnvalue (Transformation|GetWorldLocation))
  (bind _returnvalue_2 (Transformation|GetWorldLocation))
  (bind _wheelref (Variables|Default|GetWheelRef))
  (bind _playerref (Variables|Default|GetPlayerRef))
  (bind _wheelref_2 (Variables|Default|GetWheelRef))
  (bind _emmiterref (Variables|Default|GetEmmiterRef))
  (bind _returnvalue_3 (Transformation|GetVelocity _playerref))
  (bind _returnvalue_4 (Math|Vector|VectorLengthXY _returnvalue_3))
  (bind _returnvalue_5 (* _returnvalue_4 -0.03))
  (bind (_outhit _returnvalue_6) (Collision|LineTraceByChannel (Math|Vector|MakeVector (.x _returnvalue) (.y _returnvalue) (+ (.z _returnvalue) 5e+01)) (+ (Transformation|GetWorldLocation) (* (Math|Vector|GetUpVector) (* (Math|Float|MakeLiteralFloat 5e+01) -1.0))) "TraceTypeQuery1" false 0 "None"))
  (if _returnvalue_6
    (bind _output_get (Variables|Default|SetPosDelta (- (Variables|Default|GetWheelPosition) (.Distance (Collision|BreakHitResult _outhit)))))
    (Class|PrimitiveComponent|AddForceatLocation (.AsPrimitive%20Component (Utilities|Casting|CastToPrimitiveComponent (Variables|/Script/Engine.Actor|GetRootComponent (Variables|Default|GetPlayerRef)))) (* (Math|Vector|GetUpVector) (+ (* (/ (- _output_get (Variables|Default|GetPrevPosDelta)) (Utilities|Time|GetWorldDeltaSeconds)) (Variables|Default|GetDampingCoeficient)) (* _output_get (Variables|Default|GetSpringCoeficient)))) (Transformation|GetWorldLocation) "None")
    (Variables|Default|SetPrevPosDelta (Variables|Default|GetPosDelta))
    (Utilities|IsValid _wheelref
      (:Is%20Valid
        (Transformation|SetWorldLocation _wheelref (Math|Vector|MakeVector (.x _returnvalue_2) (.y _returnvalue_2) (.z (+ (.Location (Collision|BreakHitResult _outhit)) (Math|Vector|MakeVector 0.0 0.0 (Variables|Default|GetWheelMeshOffset))))) false false)
        (Utilities|IsValid _emmiterref
          (:Is%20Valid
            (Transformation|SetWorldLocation _emmiterref (+ (.Location (Collision|BreakHitResult _outhit)) "0.000000,0.000000,1.000000") false true))
          (:Is%20Not%20Valid
            _))
        (if (Variables|/Game/DriftMaster/Blueprints/BP_MainDirftController.BP_MainDirftController_C|GetHandBrake (Variables|Default|GetPlayerRef))
          (if (Variables|Default|GetRWD)
            (Transformation|AddLocalRotation _wheelref_2 (Math|Rotator|MakeRotator 0.0 0.0 0.0) false false)
            (else
              (Transformation|AddLocalRotation _wheelref_2 (Math|Rotator|MakeRotator 0.0 _returnvalue_5 0.0) false false :!label _label)))
          (elif (Variables|Default|GetRWD)
            (Transformation|AddLocalRotation _wheelref_2 (Math|Rotator|MakeRotator 0.0 (- _returnvalue_5 (/ (Math|Float|Absolute(Float) (.yaw (Variables|/Script/Engine.SceneComponent|GetRelativeRotation (Variables|/Game/DriftMaster/Blueprints/BP_MainDirftController.BP_MainDirftController_C|GetArrow (Variables|Default|GetPlayerRef))))) 5.0)) 0.0) false false)
            (else
              (goto _label))))))))